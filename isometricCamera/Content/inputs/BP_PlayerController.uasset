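; Player controller that views the game through a spawned isometric camera pawn rather than relying on the possessed pawn's view.
; BeginPlay spawns BP_IsoCameraPawn at the world origin, stores it, sets it as view target and registers the default Enhanced Input mapping context.
; On possess it re-applies that view target if the camera reference is valid.
; Debug prints report the view target or an invalid reference, plus the player pawn every tick.
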(event `self.ReceiveBeginPlay`
  (`|ExecutionSequence`
    (:`then_0`
      (bind _returnvalue (`|SpawnActorFromClass` "/Game/blueprints/BP_IsoCameraPawn.BP_IsoCameraPawn_C" (`KismetMathLibrary.MakeTransform` (0.0 0.0 0.0)) "AlwaysSpawn" "MultiplyWithRoot" null null))
      (bind _output_get (set `self.IsoCamRef` _returnvalue))
      (`self.SetViewTargetWithBlend` _output_get))
    (:`then_1`
      (`EnhancedInputSubsystemInterface.AddMappingContext` (pcsubsystem `EnhancedInputLocalPlayerSubsystem` (`GameplayStatics.GetPlayerController` 0)) "/Game/ThirdPerson/Input/IMC_Default.IMC_Default" 0 (struct)))))

(event `self.ReceivePossess`
  (params (PossessedPawn :type "Pawn Object Reference"))
  (`|ExecutionSequence`
    (:`then_0`
      (`/Engine/EditorBlueprintResources/StandardMacros.IsValid` (`self.IsoCamRef`)
        (:`Is Valid`
          (`self.SetViewTargetWithBlend` (`self.IsoCamRef`))
          (`KismetSystemLibrary.PrintString` (`KismetTextLibrary.Conv_TextToString` (`KismetTextLibrary.Conv_StringToText` (`KismetSystemLibrary.GetDisplayName` (`self.GetViewTarget`))))))
        (:`Is Not Valid`
          (`KismetSystemLibrary.PrintString` "IsoCamRef invalid"))))))

(event `self.ReceiveTick`
  (params (DeltaSeconds :type "Float (single-precision)"))
  (`KismetSystemLibrary.PrintString` (`KismetSystemLibrary.GetDisplayName` (`GameplayStatics.GetPlayerPawn` 0))))

(fn `UserConstructionScript`)